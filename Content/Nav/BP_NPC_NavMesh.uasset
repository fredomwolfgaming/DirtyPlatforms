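; An NPC pawn blueprint that wanders the navmesh at random, starting on BeginPlay.
; A self-calling NPCnav event runs AI MoveTo toward a random reachable point within a radius of the actor's current location.
; It repeats after a longer pause on success or a short one on failure, printing a debug message either way.
; An unconnected TargetPoint lookup is left in the graph, unused.
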(event Custom|NPC%20nav
  (AI|AIMoveTo self (.RandomLocation (AI|Navigation|GetRandomReachablePointinRadius (Transformation|GetActorLocation) 1e+03 0 0)) 0 5.0 false ; default is usually outside of map. also needs movement volume
    (:OnSuccess
      (Development|PrintString "move succes")
      (Utilities|FlowControl|Delay 3.0))
    (:OnFail
      (Development|PrintString "move fail")
      (Utilities|FlowControl|Delay 0.2)))
  (CallFunction|NPCNav))

(event EventBeginPlay
  (CallFunction|NPCNav) ; https://docs.unrealengine.com/4.27/en-US/InteractiveExperiences/ArtificialIntelligence/NavigationSystem/BasicNavigation/
)

(fn ConstructionScript)