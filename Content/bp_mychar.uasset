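; Player character for a target-shooting game with livestream interaction: chat messages make it jump and cheer bits fire shots or trigger hazards in timed bursts.
; Handles camera-relative movement and mouse look, and pauses animated or lerping targets it hits until the player moves.
; Firing, limited to level "1", uses a camera line trace and cosmetic bullet, advancing levels when no targets remain.
; The GameInstance handles ammo, saving, hazards and overlap pickups.
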(event Custom|ChatSent
  (params (Message%20Struct :type Twitch%20Message%20Structure))
  ;[1 1 1] Input: Jump
  (Character|Jump))

(event EventTick
  (params (DeltaSeconds :type Float%20%28single-precision%29)))

(event Collision|EventHit
  (params (MyComp :type Primitive%20Component%20Object%20Reference) (Other :type Actor%20Object%20Reference) (OtherComp :type Primitive%20Component%20Object%20Reference) (bSelfMoved :type Boolean) (HitLocation :type Vector :default "0, 0, 0") (HitNormal :type Vector :default "0, 0, 0") (NormalImpulse :type Vector :default "0, 0, 0") (Hit :type Hit%20Result%20Structure%20%28by%20ref%29))
  (bind _hitactor (Collision|BreakHitResult Hit))
  (bind _levelanimator (Variables|Default|GetLevelAnimator))
  (bind _returnvalue (Utilities|GetClass _hitactor))
  (bind _sequenceplayer (Variables|/Script/LevelSequence.LevelSequenceActor|GetSequencePlayer _levelanimator))
  ;[1 1 1] Anti-overlap prevention - does not move player version.
  (if (== _returnvalue "/Game/LerpTarget.LerpTarget_C")
    ;[1 1 1] pause Lerp movement
    (Utilities|FlowControl|Delay 0.1 :!label _label)
    (bind _aslerp_target (Utilities|Casting|CastToLerpTarget _hitactor))
    (Default|PauseLerp _aslerp_target (Math|Boolean|Equal(Boolean) (or (!= 0.0 (stale Input|AxisEvents|InputAxisleftRight AxisValue)) (!= 0.0 (stale Input|AxisEvents|InputAxisfoward AxisValue))) false))
    (if (not (or (!= 0.0 (stale Input|AxisEvents|InputAxisleftRight AxisValue)) (!= 0.0 (stale Input|AxisEvents|InputAxisfoward AxisValue)))) ; if moving, break loop
      (goto _label))
    (elif (== _returnvalue "/Game/Target.Target_C")
      ;[1 1 1] pause animator
      (Sequencer|Player|Pause _sequenceplayer)
      (Utilities|FlowControl|Delay 0.1 :!label _label_2)
      (if (or (!= 0.0 (stale Input|AxisEvents|InputAxisleftRight AxisValue)) (!= 0.0 (stale Input|AxisEvents|InputAxisfoward AxisValue)))
        (Sequencer|Player|Play _sequenceplayer :!class /Script/MovieScene.MovieSceneSequencePlayer)
        (else
          (goto _label_2))))))

(event EventBeginPlay
  ;[1 1 1] Get Game Instance actor at start, then trigger Golbal level start
  (bind _asmy_game_instance (Utilities|Casting|CastToMyGameInstance (Game|GetGameInstance)))
  (Variables|Default|SetGameInstance _asmy_game_instance)
  (Default|LevelStart(Called) _asmy_game_instance self))

(event Input|ActionEvents|InputActionjump
  (params (Key :type Key%20Structure :default "None"))
  ;[1 1 1] Input: Jump
  (:Pressed
    (if (not (Variables|/Game/MyGameInstance.MyGameInstance_C|GetIs%20Menu (Variables|Default|GetGameInstance)))
      (Character|Jump))))

(event Input|ActionEvents|InputActionexit
  (params (Key :type Key%20Structure :default "None"))
  ;[1 1 1] load title
  (:Pressed
    (Game|OpenLevel(byName) "Title")))

(event Input|AxisEvents|InputAxisfoward
  (params (AxisValue :type Float%20%28single-precision%29))
  ;[1 1 1] F/B move based on camera
  (if (not (Variables|/Game/MyGameInstance.MyGameInstance_C|GetIs%20Menu (Variables|Default|GetGameInstance)))
    (Pawn|Input|AddMovementInput (Math|Vector|GetForwardVector (Transformation|GetWorldRotation (Variables|Default|GetCamera))) AxisValue false)))

(event Input|AxisEvents|InputAxisleftRight
  (params (AxisValue :type Float%20%28single-precision%29))
  ;[1 1 1] L/R move based on camera
  (if (not (Variables|/Game/MyGameInstance.MyGameInstance_C|GetIs%20Menu (Variables|Default|GetGameInstance)))
    (Pawn|Input|AddMovementInput (Math|Vector|GetRightVector (Transformation|GetWorldRotation (Variables|Default|GetCamera))) AxisValue false)))

(event Input|AxisEvents|InputAxisrotate
  (params (AxisValue :type Float%20%28single-precision%29))
  ;[1 1 1] Rotator based on mouse
  (if (not (Variables|/Game/MyGameInstance.MyGameInstance_C|GetIs%20Menu (Variables|Default|GetGameInstance)))
    (Transformation|AddLocalRotation (Variables|Default|Getspring self) (Math|Rotator|MakeRotator 0.0 0.0 AxisValue) false false)
    (Transformation|SetActorRotation (Math|Conversions|RotationFromXVector (Math|Vector|GetForwardVector (Transformation|GetWorldRotation (Variables|Default|GetCamera)))))))

(event Input|AxisEvents|InputAxistilt
  (params (AxisValue :type Float%20%28single-precision%29))
  ;[1 1 1] Tilt up/down based on mouse
  (if (not (Variables|/Game/MyGameInstance.MyGameInstance_C|GetIs%20Menu (Variables|Default|GetGameInstance)))
    (Transformation|AddLocalRotation (Variables|Default|GetCamera) (Math|Rotator|MakeRotator 0.0 AxisValue 0.0) false false)))

(fn ConstructionScript)

(event Custom|triggerBullet
  (bind _gameinstance (Variables|Default|GetGameInstance))
  (bind _gameinstance_2 (Variables|Default|GetGameInstance))
  (bind _camera (Variables|Default|GetCamera))
  (bind _returnvalue (Transformation|GetWorldLocation _camera))
  ;[1 1 1] only use on level 1, update this to proper game mode later
  (bind _returnvalue_2 (Game|GetCurrentLevelName true))
  (if (Utilities|Enum|Equal(Enum) _returnvalue_2 "1")
    ;[1 1 1] If there is ammo remaining, then trigger a shot
    (if (!= (Variables|/Game/MyGameInstance.MyGameInstance_C|GetAmmo _gameinstance) 0)
      ;[1 1 1] Bullet Bookkeeping and sounds
      (Default|SubtractBullets _gameinstance) ; Trigger bullet bookkeeping on instance object
      (bind (_outhit _returnvalue_3) (Collision|LineTraceByChannel _returnvalue (+ _returnvalue (* (Math|Vector|GetForwardVector (Transformation|GetWorldRotation _camera)) 1e+03)) "TraceTypeQuery1" false 0 "ForOneFrame")) ; or set targets to  a NEW object type, and use LineTraceByObject
      ;[1 1 1] , then spawn a bullet to watch.
      (Game|SpawnActorfromClass "/Game/BPbullt.BPbullt_C" (|adjustdown (Transformation|GetWorldTransform (Variables|Default|GetCamera))) "Undefined" 0 0)
      ;[1 1 1] If Hit
      (if _returnvalue_3 ; save cpu time
        ;;[1 1 1] this could be replaced with an array comparison. just cheaper this way
        (switch string (Utilities|GetClassDisplayName (Utilities|GetClass (.HitActor (Collision|BreakHitResult _outhit))))
          (:Target_C
            _)
          (:LerpTarget_C
            _))
        (Actor|DestroyActor (.HitActor (Collision|BreakHitResult _outhit))) ; destory target
        ;;[1 1 1] find out how many targets are left
        (bind _outactors (Actor|GetAllActorsOfClass "/Game/Target.Target_C"))
        (bind _outactors_2 (Actor|GetAllActorsOfClass "/Game/LerpTarget.LerpTarget_C"))
        ;;[1 1 1] If that was the last target?
        (if (== (+ (Utilities|Array|Length _outactors) (Utilities|Array|Length _outactors_2)) 0)
          ;;[1 1 1] If so, then Save the game
          (Default|Save/LoadGame _gameinstance_2 true)
          ;;[1 1 1] Find out if that was the last level
          (bind _returnvalue_4 (Game|GetCurrentLevelName true))
          (if (== (Variables|/Game/MyGameInstance.MyGameInstance_C|GetTOTAL_LEVELS _gameinstance_2) (Math|Conversions|ToInteger(Byte) _returnvalue_4))
            ;;[1 1 1] If that was the final level, then load win screen, else increment and load
            (Variables|/Game/MyGameInstance.MyGameInstance_C|SetHasWon _gameinstance_2 true)
            (Game|OpenLevel(byName) "LossWin")
            (else
              (Game|OpenLevel(byName) (Utilities|String|StringToName (Utilities|String|ToString(Integer) (+ (Math|Conversions|ToInteger(Byte) _returnvalue_4) 1)))) ; proceed to next level if there is one
            ))))
      (else
        (Development|PrintString "Click click. Dry firing can damage your weapon.") ; play dry fire click sound
      ))))

(event Input|ActionEvents|InputActionFire
  (params (Key :type Key%20Structure :default "None"))
  (bind _gameinstance (Variables|Default|GetGameInstance))
  (bind _gameinstance_2 (Variables|Default|GetGameInstance))
  (bind _camera (Variables|Default|GetCamera))
  (bind _returnvalue (Transformation|GetWorldLocation _camera))
  (:Pressed
    ;[1 1 1] only use on level 1, update this to proper game mode later
    (bind _returnvalue_2 (Game|GetCurrentLevelName true))
    (if (Utilities|Enum|Equal(Enum) _returnvalue_2 "1")
      ;[1 1 1] If there is ammo remaining, then trigger a shot
      (if (!= (Variables|/Game/MyGameInstance.MyGameInstance_C|GetAmmo _gameinstance) 0)
        ;[1 1 1] Bullet Bookkeeping and sounds
        (Default|SubtractBullets _gameinstance) ; Trigger bullet bookkeeping on instance object
        (bind (_outhit _returnvalue_3) (Collision|LineTraceByChannel _returnvalue (+ _returnvalue (* (Math|Vector|GetForwardVector (Transformation|GetWorldRotation _camera)) 1e+03)) "TraceTypeQuery1" false 0 "ForOneFrame")) ; or set targets to  a NEW object type, and use LineTraceByObject
        ;[1 1 1] , then spawn a bullet to watch.
        (Game|SpawnActorfromClass "/Game/BPbullt.BPbullt_C" (|adjustdown (Transformation|GetWorldTransform (Variables|Default|GetCamera))) "Undefined" 0 0)
        ;[1 1 1] If Hit
        (if _returnvalue_3 ; save cpu time
          ;;[1 1 1] this could be replaced with an array comparison. just cheaper this way
          (switch string (Utilities|GetClassDisplayName (Utilities|GetClass (.HitActor (Collision|BreakHitResult _outhit))))
            (:Target_C
              _)
            (:LerpTarget_C
              _))
          (Actor|DestroyActor (.HitActor (Collision|BreakHitResult _outhit))) ; destory target
          ;;[1 1 1] find out how many targets are left
          (bind _outactors (Actor|GetAllActorsOfClass "/Game/Target.Target_C"))
          (bind _outactors_2 (Actor|GetAllActorsOfClass "/Game/LerpTarget.LerpTarget_C"))
          ;;[1 1 1] If that was the last target?
          (if (== (+ (Utilities|Array|Length _outactors) (Utilities|Array|Length _outactors_2)) 0)
            ;;[1 1 1] If so, then Save the game
            (Default|Save/LoadGame _gameinstance_2 true)
            ;;[1 1 1] Find out if that was the last level
            (bind _returnvalue_4 (Game|GetCurrentLevelName true))
            (if (== (Variables|/Game/MyGameInstance.MyGameInstance_C|GetTOTAL_LEVELS _gameinstance_2) (Math|Conversions|ToInteger(Byte) _returnvalue_4))
              ;;[1 1 1] If that was the final level, then load win screen, else increment and load
              (Variables|/Game/MyGameInstance.MyGameInstance_C|SetHasWon _gameinstance_2 true)
              (Game|OpenLevel(byName) "LossWin")
              (else
                (Game|OpenLevel(byName) (Utilities|String|StringToName (Utilities|String|ToString(Integer) (+ (Math|Conversions|ToInteger(Byte) _returnvalue_4) 1)))) ; proceed to next level if there is one
              ))))
        (else
          (Development|PrintString "Click click. Dry firing can damage your weapon.") ; play dry fire click sound
        )))))

(event Custom|CheerSent
  (params (cheer%20struct :type Twitch%20Cheer%20Structure))
  (bind (_message _bits) (Utilities|Struct|BreakTwitchCheer cheer%20struct))
  ;[1 1 1] cheer ingest
  (if (not (Variables|/Game/MyGameInstance.MyGameInstance_C|GetIs%20Menu (Variables|Default|GetGameInstance)))
    ;[1 1 1] check ammo
    (if (>= _bits (Variables|/Game/MyGameInstance.MyGameInstance_C|GetAmmo (Variables|Default|GetGameInstance))) ; if larger than max ammo
      ;[1 1 1] delayed per increment for loop, remainder is in shots
      (Variables|Default|SetBurst%20counter (/ _bits 10)) ; input last index of for loop, aka how many shots
      (Default|Trigger:Hazard (Variables|Default|GetGameInstance) :!label _label)
      (Utilities|FlowControl|Delay 0.1)
      (bind _result (Math|Integer|DecrementInt (Variables|Default|GetBurst%20counter))
        (:%20%20
          (if (== _result 0)
            (Variables|Default|SetBurst%20counter (Math|Integer|%(Integer) _bits 10)) ; whats left after dividing by 10 is bullets
            (else
              (goto _label)))))
      (else
        ;[1 1 1] delayed per increment for loop
        (Variables|Default|SetBurst%20counter _bits) ; input last index of for loop, aka how many shots
      ))
    (CallFunction|TriggerBullet :!label _label_2)
    (Utilities|FlowControl|Delay 0.2)
    (bind _result_2 (Math|Integer|DecrementInt (Variables|Default|GetBurst%20counter))
      (:%20%20
        (if (not (== _result_2 0))
          (goto _label_2))))))

(event Collision|EventActorBeginOverlap
  (params (OtherActor :type Actor%20Object%20Reference))
  (bind _gameinstance (Variables|Default|GetGameInstance))
  ;[1 1 1] Trigger activations: switch based on the blueprint class name of the interacted object ( BlueprintClassname + "_C" )
  (switch string (Utilities|GetClassDisplayName (Utilities|GetClass OtherActor))
    (:KillingFloor_C
      (Default|RestartNon-menuLevel _gameinstance))
    (:DangerCone_C
      (Default|Trigger:Hazard _gameinstance)
      (Character|Jump))
    (:AmmoCrate_C
      (Default|AmmoBox _gameinstance OtherActor false))
    (:Keys_C
      (Default|KeyGet _gameinstance OtherActor))))